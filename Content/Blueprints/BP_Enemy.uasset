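; BP_Enemy is an enemy ship actor that gets a randomized two-tone look and a scale-in effect when spawned.
; The SetColor event creates a dynamic instance of M_Base_Ship, sets random body and wing colors from small fixed palettes, and applies it to the ship mesh.
; It then plays a timeline that drives the actor's scale.
; BeginPlay, overlap and Tick are unused, and nothing in this graph calls SetColor.
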(event `self.SetColor`
  (set `self.BodyColorIndex` (`KismetMathLibrary.RandomIntegerInRange` 0 3))
  (set `self.WingColorIndex` (`KismetMathLibrary.RandomIntegerInRange` 0 3))
  (bind _returnvalue (`KismetMaterialLibrary.CreateDynamicMaterialInstance` "/Game/SpaceshipBattle/Materials/M_Base_Ship.M_Base_Ship"))
  (`MaterialInstanceDynamic.SetVectorParameterValue` _returnvalue "Color1" (select `int` (`self.BodyColorIndex`) :`0` (struct :`R` 0.204847 :`G` 0.833333 :`B` 0.232003 :`A` 1.0) :`1` (struct :`R` 0.199593 :`G` 0.263866 :`B` 0.833333 :`A` 1.0) :`2` (struct :`R` 0.770833 :`G` 0.316181 :`B` 0.184624 :`A` 1.0) :`3` (struct :`R` 0.869792 :`G` 0.766124 :`B` 0.160882 :`A` 1.0) :!type "LinearColor Structure"))
  (`MaterialInstanceDynamic.SetVectorParameterValue` _returnvalue "Color2" (select `int` (`self.WingColorIndex`) :`0` (struct :`R` 0.833333 :`G` 0.190445 :`B` 0.784598 :`A` 1.0) :`1` (struct :`R` 0.259365 :`G` 0.800155 :`B` 0.833333 :`A` 1.0) :`2` (struct :`R` 0.498161 :`G` 0.770833 :`B` 0.240824 :`A` 1.0) :`3` (struct :`R` 0.827668 :`G` 0.869792 :`B` 0.821001 :`A` 1.0) :!type "LinearColor Structure"))
  (`PrimitiveComponent.SetMaterial` (`self.ShipSM`) 0 _returnvalue)
  (bind (_direction _scale) (`Timeline|SpawnScaleTimeLine`)
    (:`Update`
      (`self.SetActorScale3D` (`KismetMathLibrary.Conv_DoubleToVector` _scale)))))

(fn `UserConstructionScript`)